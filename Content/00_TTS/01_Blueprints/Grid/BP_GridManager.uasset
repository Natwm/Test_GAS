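; Grid manager actor that spawns a tile grid from the world on BeginPlay and marks the tile under the cursor with a debug sphere each tick.
; World spawning and cursor lookup are defined outside this graph.
; SpawnGrid, not called here, rebuilds GridHolder instances centred on GridCenter, which it resets to the origin.
; Tiles are scaled to GridTileSize using the mesh's X bound as both height and width.
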(event `self.ReceiveBeginPlay`
  (`self.SpawnGridFromWorld`))

(event `self.ReceiveTick`
  (params (DeltaSeconds :type "Float (single-precision)"))
  (bind _returnvalue (`self.GetTileLocationUnderCursor`))
  (`KismetSystemLibrary.DrawDebugSphere` _returnvalue 10.0 12 (struct :`R` 0.981855 :`G` 1.0 :`A` 1.0)))

(event `Key|A`
  (params (Key :type "Key Structure")))

(fn `FindAndStoreTileSizeBP`
  (bind _output_get (set `self.TileHeight` (* (.x (`.BoxExtent` (`KismetMathLibrary.BreakBoxSphereBounds` (`StaticMesh.GetBounds` (`StaticMeshComponent.StaticMesh` (`self.GridHolder`)))))) 2.0)))
  (set `self.TileWidth` _output_get))

(fn `GetBottomLeftTileAndCenter`
  (returns (Center :type "Vector Structure") (BottomLeft :type "Vector Structure"))
  (return (0.0 0.0 0.0) (- (`self.GridCenter`) (* (/ (- (`self.GridSize`) (`KismetMathLibrary.MakeVector2D` (`KismetMathLibrary.SelectFloat` 0.0 1.0) (`KismetMathLibrary.SelectFloat` 0.0 1.0))) 2.0) (`KismetMathLibrary.Conv_VectorToVector2D` (`self.GridTileSize`))))))

(fn `SpawnGrid`
  (locals (BottomLeftTile :type "Vector Structure" :default (0.0 0.0 0.0)) (XIndex :type Integer) (YIndex :type Integer))
  (bind (_gridsize_x _gridsize_y) (`KismetMathLibrary.BreakVector2D` (`self.GridSize`)))
  (bind (_gridsize_x_2 _gridsize_y_2) (`KismetMathLibrary.BreakVector2D` (`self.GridSize`)))
  (bind _gridsize_x_3 (`KismetMathLibrary.BreakVector2D` (`self.GridSize`)))
  (`self.FindAndStoreTileSizeBP`)
  (if (> (* _gridsize_x _gridsize_y) 0.0)
    (`InstancedStaticMeshComponent.ClearInstances` (`self.GridHolder`))
    (bind (_center _bottomleft) (`self.GetBottomLeftTileAndCenter`))
    (set `self.GridCenter` _center)
    (set `local.BottomLeftTile` _bottomleft)
    (for _index (range (+ (`KismetMathLibrary.FTrunc` (- _gridsize_x_3 1.0)) 1))
      (set `local.XIndex` _index)
      (for _index_2 (range (+ (`KismetMathLibrary.FTrunc` (- _gridsize_y_2 1.0)) 1))
        (set `local.YIndex` _index_2)
        (`InstancedStaticMeshComponent.AddInstance` (`self.GridHolder`) (`KismetMathLibrary.MakeTransform` (+ (`local.BottomLeftTile`) (* (`self.GridTileSize`) (`KismetMathLibrary.MakeVector` (`KismetMathLibrary.Conv_IntToDouble` (`local.XIndex`)) (`KismetMathLibrary.Conv_IntToDouble` (`local.YIndex`)) 1.0))) (struct) (/ (`self.GridTileSize`) (`KismetMathLibrary.MakeVector` (`self.TileHeight`) (`self.TileWidth`) 1.0))) false)))))

(fn `UserConstructionScript`)